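; H4HGameMode is a game mode Blueprint that routes step-based progression for the game's levels.
; BeginPlay caches the H4HGameInstance, which holds the level number and current step.
; The H4HNextStep event switches on the level number and, for level 1, passes the current step to Scene1.
; Scene1 switches on that step but has no case logic yet.
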(event Custom|H4HNextStep
  (bind _h4hgame_instance (Variables|Default|GetH4HGame%20Instance))
  (switch int (Variables|/Game/Blueprints/H4HGameInstance.H4HGameInstance_C|GetLevelNum _h4hgame_instance)
    (:1
      (Utilities|Scene1 (Variables|/Game/Blueprints/H4HGameInstance.H4HGameInstance_C|GetCurrentStep _h4hgame_instance)))))

(event EventBeginPlay
  ;[1 1 1] Begin Play
  (bind _ash4hgame_instance (Utilities|Casting|CastToH4HGameInstance (Game|GetGameInstance)))
  (Variables|Default|SetH4HGame%20Instance _ash4hgame_instance))

(event EventTick
  (params (DeltaSeconds :type Float%20%28single-precision%29)))

(fn ConstructionScript)