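; MoneyBin is a sorting bin that fills as actors tagged "Money" are placed in it, as part of a game-mode step.
; Overlap begin and end raise or lower the progress bar on its widget, which receives the bin's name and division count at BeginPlay.
; A nearly full bar marks the bin done and checks the MoneyBins array, completing the H4H step when all are done.
; The code that would populate that array is disconnected.
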(event OnComponentBeginOverlap(Bin)
  (params (OverlappedComponent :type Primitive%20Component%20Object%20Reference) (OtherActor :type Actor%20Object%20Reference) (OtherComp :type Primitive%20Component%20Object%20Reference) (OtherBodyIndex :type Integer) (bFromSweep :type Boolean) (SweepResult :type Hit%20Result%20Structure%20%28by%20ref%29))
  (bind _money_bin_widget (Variables|Default|GetMoney%20Bin%20Widget))
  (if (!= (Utilities|Array|FindItem (Variables|/Script/Engine.Actor|GetTags OtherActor) "Money") -1)
    (Default|UpdateProgressBar _money_bin_widget true)
    (bind _percent (Default|GetBarsPercent _money_bin_widget))
    (if (> _percent 0.98)
      (Variables|Default|SetSet%20Done true)
      (CallFunction|Allmoniescompleted))))

(event OnComponentEndOverlap(Bin)
  (params (OverlappedComponent :type Primitive%20Component%20Object%20Reference) (OtherActor :type Actor%20Object%20Reference) (OtherComp :type Primitive%20Component%20Object%20Reference) (OtherBodyIndex :type Integer))
  (bind _money_bin_widget (Variables|Default|GetMoney%20Bin%20Widget))
  (if (!= (Utilities|Array|FindItem (Variables|/Script/Engine.Actor|GetTags OtherActor) "Money") -1)
    (Default|UpdateProgressBar _money_bin_widget false)
    (bind _percent (Default|GetBarsPercent _money_bin_widget))
    (if (< _percent 0.98)
      (Variables|Default|SetSet%20Done false))))

(event EventBeginPlay
  (bind _asmoney_bin_widget (Utilities|Casting|CastToMoneyBinWidget (UserInterface|GetUserWidgetObject (Variables|Default|GetWidget))))
  (bind _output_get (Variables|Default|SetMoney%20Bin%20Widget _asmoney_bin_widget))
  (Variables|/Game/Blueprints/Trent/UI/Scene1/MoneyBinWidget.MoneyBinWidget_C|SetDivisions _output_get (Variables|MoneyBin|GetMoneyAmount))
  (Rendering|Material|SetScalarParameterValueonMaterials (Variables|Default|GetBin) "Opacity" 0.7)
  (Variables|/Game/Blueprints/Trent/UI/Scene1/MoneyBinWidget.MoneyBinWidget_C|SetBin%20Name _output_get (Variables|MoneyBin|GetBin%20Name)))

(event Collision|EventActorBeginOverlap
  (params (OtherActor :type Actor%20Object%20Reference)))

(event EventTick
  (params (DeltaSeconds :type Float%20%28single-precision%29)))

(fn ConstructionScript)

(fn Allmoniescompleted
  (bind _array_element (Utilities|Array|ForEachLoopwithBreak (Variables|Default|GetMoneyBins) :!label _label)
    (:LoopBody
      (bind _output_get (LocalVariables|SetAll%20done (Variables|MoneyBin_C|GetSet%20Done _array_element)))
      (if (not _output_get)
        (goto _label Break)))
    (:Completed
      (if (LocalVariables|GetAll%20done)
        (Utilities|H4HCompleteStep (Game|GetGameMode))))))