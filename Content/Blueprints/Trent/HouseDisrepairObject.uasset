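; House disrepair object that the player can pay to repair, counting toward a game mode step.
; Collision overlap arms the purchase input and shows a prompt widget, turned toward the camera by a looping timer.
; Repairing passes the cost to the player, hides the prompt, then scans actors tagged HouseAppliances to complete the step.
; That scan overwrites its flag each iteration, so only the last actor's state decides completion.
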(event OnComponentBeginOverlap(Collision)
  (params (OverlappedComponent :type Primitive%20Component%20Object%20Reference) (OtherActor :type Actor%20Object%20Reference) (OtherComp :type Primitive%20Component%20Object%20Reference) (OtherBodyIndex :type Integer) (bFromSweep :type Boolean) (SweepResult :type Hit%20Result%20Structure%20%28by%20ref%29))
  ;[1 1 1] Set House repair object active
  (Variables|RepairObject|SetIsActive true)
  (if (not (Variables|RepairObject|GetRepaired))
    (Development|SetHiddeninGame (Variables|Default|GetWidget) false false)
    (Utilities|Time|SetTimerbyFunctionName 0 "UpdateUIRotation" 0.01 true)))

(event OnComponentEndOverlap(Collision)
  (params (OverlappedComponent :type Primitive%20Component%20Object%20Reference) (OtherActor :type Actor%20Object%20Reference) (OtherComp :type Primitive%20Component%20Object%20Reference) (OtherBodyIndex :type Integer))
  ;[1 1 1] Set House repair object active
  (Variables|RepairObject|SetIsActive false)
  (Development|SetHiddeninGame (Variables|Default|GetWidget) true false)
  (Utilities|Time|ClearTimerbyFunctionName 0 "UpdateUIRotation"))

(event EventBeginPlay)

(event Collision|EventActorBeginOverlap
  (params (OtherActor :type Actor%20Object%20Reference)))

(event EventTick
  (params (DeltaSeconds :type Float%20%28single-precision%29)))

(event Input|ActionEvents|InputActionPurchaseRepair
  (params (Key :type Key%20Structure :default "None"))
  ;[1 1 1] Repair
  (:Pressed
    (if (and (Variables|RepairObject|GetIsActive) (not (Variables|RepairObject|GetRepaired)))
      (Default|RepairItem (Variables|Default|GetPlayerREF) (Variables|RepairObject|GetCost))
      (Variables|RepairObject|SetRepaired true)
      (Development|SetHiddeninGame (Variables|Default|GetWidget) true false)
      (CallFunction|CheckifAllThingsrepaired))))

(fn ConstructionScript)

(fn UpdateUIRotation
  (bind _widget (Variables|Default|GetWidget))
  (Transformation|SetWorldRotation _widget (Math|Rotator|FindLookatRotation (Transformation|GetWorldLocation _widget) (Camera|GetCameraLocation (Game|GetPlayerCameraManager 0))) false false))

(fn CheckifAllThingsrepaired
  (bind _outactors (Actor|GetAllActorswithTag "HouseAppliances"))
  (for _array_element _outactors
    (bind _ashouse_disrepair_object (Utilities|Casting|CastToHouseDisrepairObject _array_element))
    (LocalVariables|SetAll%20Repaired? (Variables|HouseDisrepairObject_C|GetRepaired _ashouse_disrepair_object)))
  (if (LocalVariables|GetAll%20Repaired?)
    (Utilities|H4HCompleteStep (Game|GetGameMode))))