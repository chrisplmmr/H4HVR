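; FrameStructure_1 is a building-piece actor that settles into a level pose and can show a colored highlight.
; Two seconds after BeginPlay, ToggleOnOff flips actor tick and updates physics simulation.
; While ticking, a near-zero pitch triggers a one-time physics stop, pitch snap, tick shutdown and Setup flag.
; Highlight functions add or destroy a collision-free mesh copy using dynamic emissive materials.
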(event EventBeginPlay
  ;[1 0.2393 0.2592] Begin Play
  (Utilities|FlowControl|Delay 2.0)
  (CallFunction|ToggleonOff))

(event EventTick
  (params (DeltaSeconds :type Float%20%28single-precision%29))
  (bind _buildingpiece (Variables|Default|GetBuildingPiece))
  (bind _relativerotation (Variables|/Script/Engine.SceneComponent|GetRelativeRotation _buildingpiece))
  ;[1 1 1] Move this out of event tick into timer function, like above
  (if (Math|Float|NearlyEqual(Float) (.pitch (Variables|/Script/Engine.SceneComponent|GetRelativeRotation (Variables|Default|GetBuildingPiece))) 0.0 2.0)
    (Utilities|FlowControl|DoOnce false
      (:Completed
        (Physics|SetSimulatePhysics (Variables|Default|GetBuildingPiece) false)
        (Transformation|SetRelativeRotation _buildingpiece (Math|Rotator|MakeRotator (.roll _relativerotation) 0.0 (.yaw _relativerotation)) false false)
        (Actor|Tick|SetActorTickEnabled false)
        (Variables|Default|SetSetup true)))))

(fn ConstructionScript)

(fn CheckifSet)

(fn CreateHighlight
  (params (Higlight%20Color :type Linear%20Color%20Structure :default "(R=0.160689,G=0.697539,B=0.989583,A=1.000000)"))
  (bind _buildingpiece (Variables|Default|GetBuildingPiece))
  (bind _returnvalue (AddComponent|AddStaticMeshComponent false (Transformation|GetRelativeTransform _buildingpiece)))
  (Components|StaticMesh|SetStaticMesh _returnvalue (Variables|/Script/Engine.StaticMeshComponent|GetStaticMesh _buildingpiece))
  (bind _output_get (Variables|Default|SetHighlight%20Mesh _returnvalue))
  (Collision|SetCollisionEnabled _output_get "NoCollision")
  ;[1 1 1] Set Material to be the highlight material
  (for _index (range 0 (- (Rendering|Material|GetNumMaterials _returnvalue) 1))
    (bind _returnvalue_2 (Rendering|Material|CreateDynamicMaterialInstance _returnvalue _index "/Game/Assets/Trent/Materials/EmmissiveHighlight.EmmissiveHighlight" "None" :!class /Script/Engine.PrimitiveComponent))
    (Rendering|Material|SetVectorParameterValue _returnvalue_2 "Color" Higlight%20Color :!class /Script/Engine.MaterialInstanceDynamic)))

(fn DeleteHighlight
  (bind _highlight_mesh (Variables|Default|GetHighlight%20Mesh))
  (Utilities|IsValid _highlight_mesh
    (:Is%20Valid
      (Components|DestroyComponent _highlight_mesh))))

(fn ToggleonOff
  (bind _returnvalue (Class|Actor|IsActorTickEnabled))
  (bind _returnvalue_2 (not _returnvalue))
  (Actor|Tick|SetActorTickEnabled _returnvalue_2)
  (Physics|SetSimulatePhysics (Variables|Default|GetBuildingPiece) _returnvalue_2))