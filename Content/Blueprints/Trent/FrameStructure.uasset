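; FrameStructure is a building piece that locks in place once it is upright or level on the pitch axis.
; Tick checks the BuildingPiece relative pitch and, the first time it nears zero, stops physics simulation and snaps pitch to zero, keeping roll and yaw.
; A hit sets IsBeingmoved, which nothing reads.
; A planned move from Tick to a timer is unfinished: the timer call is unwired and CheckIfSet is empty.
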(event OnComponentHit(BuildingPiece)
  (params (HitComponent :type Primitive%20Component%20Object%20Reference) (OtherActor :type Actor%20Object%20Reference) (OtherComp :type Primitive%20Component%20Object%20Reference) (NormalImpulse :type Vector :default "0, 0, 0") (Hit :type Hit%20Result%20Structure%20%28by%20ref%29))
  (Variables|Default|SetIsBeingmoved true))

(event OnComponentBeginOverlap(BuildingPiece)
  (params (OverlappedComponent :type Primitive%20Component%20Object%20Reference) (OtherActor :type Actor%20Object%20Reference) (OtherComp :type Primitive%20Component%20Object%20Reference) (OtherBodyIndex :type Integer) (bFromSweep :type Boolean) (SweepResult :type Hit%20Result%20Structure%20%28by%20ref%29)))

(event OnComponentEndOverlap(BuildingPiece)
  (params (OverlappedComponent :type Primitive%20Component%20Object%20Reference) (OtherActor :type Actor%20Object%20Reference) (OtherComp :type Primitive%20Component%20Object%20Reference) (OtherBodyIndex :type Integer)))

(event EventBeginPlay)

(event Collision|EventActorBeginOverlap
  (params (OtherActor :type Actor%20Object%20Reference)))

(event EventTick
  (params (DeltaSeconds :type Float%20%28single-precision%29))
  (bind _buildingpiece (Variables|Default|GetBuildingPiece))
  (bind _relativerotation (Variables|/Script/Engine.SceneComponent|GetRelativeRotation _buildingpiece))
  ;[1 1 1] Move this out of event tick into timer function, like above
  (if (Math|Float|NearlyEqual(Float) (.pitch (Variables|/Script/Engine.SceneComponent|GetRelativeRotation (Variables|Default|GetBuildingPiece))) 0.0 2.0)
    (Utilities|FlowControl|DoOnce false
      (:Completed
        (Physics|SetSimulatePhysics (Variables|Default|GetBuildingPiece) false)
        (Transformation|SetRelativeRotation _buildingpiece (Math|Rotator|MakeRotator (.roll _relativerotation) 0.0 (.yaw _relativerotation)) false false)))))

(fn ConstructionScript)

(fn CheckifSet)